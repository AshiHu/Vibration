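; BP_FallingRock is a looping hazard rock that kills BP_mouse2 on overlap while falling.
; Tick moves the Scene component down at FallingSpeed and sphere-traces for impact, with Size driving both trace radius and construction-time scale.
; Impact hides the rock, stops Tick, triggers camera shake, earthquake sound and Niagara meteor effect, then starts a timer to return it to its origin after ResetTime.
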(event `self.ReceiveBeginPlay`
  (`self.ResetRock`))

(event `self.ReceiveTick`
  (params (DeltaSeconds :type "Float (single-precision)"))
  (bind _returnvalue (`SceneComponent.K2_GetComponentLocation` (`self.Scene`)))
  (`SceneComponent.K2_AddWorldOffset` (`self.Scene`) (`KismetMathLibrary.MakeVector` 0.0 0.0 (* (`GameplayStatics.GetWorldDeltaSeconds`) (`self.FallingSpeed`) -1.0)) false false)
  (bind (_outhit _returnvalue_2) (`KismetSystemLibrary.SphereTraceSingle` _returnvalue (+ _returnvalue (0.0 0.0 -1.0)) (- (`self.Size`) 5.0) "TraceTypeQuery1"))
  (if _returnvalue_2
    (`SceneComponent.SetHiddenInGame` (`self.Scene`) true true)
    (`self.SetActorTickEnabled` false)
    (`KismetSystemLibrary.K2_SetTimerDelegate` (`|CreateDelegate` :!event `ResetRock`) (`self.ResetTime`))
    (`GameplayStatics.PlayWorldCameraShake` "/Game/character/CS_ShakeNormal.CS_ShakeNormal_C" (`SceneComponent.K2_GetComponentLocation` (`self.Scene`)) 0.0 1000.0)
    (set `self.isFalling` false)
    (`AudioComponent.Play` (`self.423120__ogsoundfx__earthquake-1-big_Cue`) 0.0)
    (`NiagaraFunctionLibrary.SpawnSystemAtLocation` "/Game/particle/NS_Meteor.NS_Meteor" (`SceneComponent.K2_GetComponentLocation` (`self.Scene`)))))

(event `ResetRock`
  (`SceneComponent.SetHiddenInGame` (`self.Scene`) false true)
  (`self.SetActorTickEnabled` true)
  (`SceneComponent.K2_SetRelativeLocation` (`self.Scene`) (0.0 0.0 0.0) false false)
  (set `self.isFalling` true))

(event `self.Sphere1.OnComponentBeginOverlap`
  (params (OverlappedComponent :type "PrimitiveComponent Object Reference") (OtherActor :type "Actor Object Reference") (OtherComp :type "PrimitiveComponent Object Reference") (OtherBodyIndex :type Integer) (bFromSweep :type Boolean) (SweepResult :type "HitResult Structure (by ref)"))
  (bind _asbp_mouse_2 (cast `/Game/character/BP_mouse2` OtherActor))
  (if (`self.isFalling`)
    (`/Game/character/BP_mouse2.Death` _asbp_mouse_2)))

(fn `UserConstructionScript`
  (`SceneComponent.SetRelativeScale3D` (`self.Scene`) (`KismetMathLibrary.Conv_DoubleToVector` (/ (`self.Size`) 50.0))))