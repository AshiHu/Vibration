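; BP_mouse2 is a character that moves by charged launches along a steerable arrow's forward direction while on walkable floor.
; Steering yaws the arrow at a rate proportional to speed and nudges velocity by a small fraction of that turn.
; Each tick aligns the cube to floor normal and arrow heading, with the spring arm easing after it.
; A short forward sphere trace relaunches the character off obstacles along the mirrored heading with upward lift.
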(event `self.ReceiveBeginPlay`
  (`EnhancedInputSubsystemInterface.AddMappingContext` (pcsubsystem `EnhancedInputLocalPlayerSubsystem` (`GameplayStatics.GetPlayerController` 0)) "/Game/character/IMP_Inputs.IMP_Inputs" 0 (struct)))

(event `self.ReceiveTick`
  (params (DeltaSeconds :type "Float (single-precision)"))
  (bind _returnvalue (`SceneComponent.K2_GetComponentLocation` (`self.CapsuleComponent`)))
  (bind (_currentfloor_bblockinghit _currentfloor_bwalkablefloor _currentfloor_blinetrace _currentfloor_floordist _currentfloor_linedist _currentfloor_hitresult) (break `FindFloorResult` (`CharacterMovementComponent.CurrentFloor` (`self.CharacterMovement`))))
  (bind _returnvalue_2 (`KismetMathLibrary.MakeRotFromZX` (select `bool` _currentfloor_bblockinghit :`false` (0.0 0.0 1.0) :`true` (`.ImpactNormal` (`GameplayStatics.BreakHitResult` _currentfloor_hitresult))) (`SceneComponent.GetForwardVector` (`self.Arrow1`))))
  (`SceneComponent.K2_SetWorldRotation` (`self.SpringArm`) (`KismetMathLibrary.RInterpTo` (`SceneComponent.K2_GetComponentRotation` (`self.SpringArm`)) _returnvalue_2 (`GameplayStatics.GetWorldDeltaSeconds`) (`self.CameraSpeed`)) false false)
  (`SceneComponent.K2_SetWorldRotation` (`self.Cube`) _returnvalue_2 false false)
  (bind (_outhit _returnvalue_3) (`KismetSystemLibrary.SphereTraceSingle` _returnvalue (+ _returnvalue (* (`KismetMathLibrary.GetForwardVector` _returnvalue_2) 15.0)) 20.0 "TraceTypeQuery1"))
  (if _returnvalue_3
    (`self.LaunchCharacter` (+ (* (`KismetMathLibrary.MirrorVectorByNormal` (`SceneComponent.GetForwardVector` (`self.Arrow1`)) (`.Normal` (`GameplayStatics.BreakHitResult` _outhit))) 500.0) (0.0 0.0 500.0)) true true)))

(event `EnhancedInput|/Game/character/IA_Launch`
  (params (ActionValue :type Boolean) (ElapsedSeconds :type "Float (double-precision)") (TriggeredSeconds :type "Float (double-precision)") (InputAction :type "InputAction Object Reference" :default "/Game/character/IA_Launch.IA_Launch"))
  (bind (_currentfloor_bblockinghit _currentfloor_bwalkablefloor) (break `FindFloorResult` (`CharacterMovementComponent.CurrentFloor` (`self.CharacterMovement`))))
  (bind _returnvalue (`KismetMathLibrary.Lerp` (`self.MinLaunch`) (`self.MaxLaunch`) (`KismetMathLibrary.FMin` (/ ElapsedSeconds (`self.ChargeTime`)) 1.0)))
  (:`Triggered`
    (`KismetSystemLibrary.PrintString` (`KismetStringLibrary.Conv_DoubleToString` _returnvalue)))
  (:`Completed`
    (if _currentfloor_bwalkablefloor
      (`self.LaunchCharacter` (* (`SceneComponent.GetForwardVector` (`self.Arrow1`)) _returnvalue) true))))

(event `EnhancedInput|/Game/character/IA_Dir`
  (params (ActionValue :type "Vector2D Structure") (ElapsedSeconds :type "Float (double-precision)") (TriggeredSeconds :type "Float (double-precision)") (InputAction :type "InputAction Object Reference" :default "/Game/character/IA_Dir.IA_Dir"))
  (bind _returnvalue (`KismetMathLibrary.Vector_Up`))
  (bind _charactermovement (`self.CharacterMovement`))
  (bind _returnvalue_2 (* ActionValue_Y (`GameplayStatics.GetWorldDeltaSeconds`) (/ (`KismetMathLibrary.VSize` (`MovementComponent.Velocity` (`self.CharacterMovement`))) 5.0)))
  (:`Triggered`
    (`SceneComponent.K2_SetWorldRotation` (`self.Arrow1`) (`KismetMathLibrary.MakeRotFromZX` _returnvalue (`KismetMathLibrary.RotateAngleAxis` (`SceneComponent.GetForwardVector` (`self.Arrow1`)) _returnvalue_2 _returnvalue)) false false)
    (set `MovementComponent.Velocity` (`KismetMathLibrary.RotateAngleAxis` (`MovementComponent.Velocity` _charactermovement) (* _returnvalue_2 0.01) _returnvalue) _charactermovement)))

(fn `UserConstructionScript`)